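; Ranged AI enemy character that fights with a rifle, extending a parent character's begin-play and attack logic.
; On BeginPlay it spawns a rifle, attaches it to a hand socket and signals that the weapon is equipped.
; Attacking plays a fire montage whose notify fires a blockable bullet through BPAttacksComponent at a valid target, ending on completion or interruption.
; It also supplies its own combat ranges and walk speeds per movement state.
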(event EventBeginPlay
  (|CallParentFunction)
  (CallFunction|EquipWeapon))

(event EventAttack
  (params (AttackTarget :type Actor%20Object%20Reference))
  (|CallParentFunction AttackTarget)
  (bind _notifyname (Animation|Montage|PlayMontage (Variables|Character|GetMesh) "/Game/Mannequin/Animations/AM_Fire_Rifle_Ironsights.AM_Fire_Rifle_Ironsights")
    (:OnCompleted
      (CallFunction|AttackEnd AttackTarget :!label _label))
    (:OnInterrupted
      (goto _label))
    (:OnNotifyBegin
      (switch name _notifyname
        (:Fire
          (Utilities|IsValid AttackTarget
            (:Is%20Valid
              (Default|FireBullet (Variables|Default|GetBP_AttacksComponent) (Transformation|GetActorLocation (Variables|Default|GetWeaponActor)) (Transformation|GetActorLocation AttackTarget) (Utilities|Struct|MakeS_DamageInfo 15.0 "NewEnumerator2" "NewEnumerator0" false true)))))))))

(event EventEquipWeapon
  (bind _returnvalue (Game|SpawnActorfromClass "/Game/Gameplay/Weapons/BP_WeaponRifle.BP_WeaponRifle_C" (Math|Transform|MakeTransform "0, 0, 0") "Undefined" "MultiplyWithRoot" 0 0))
  (bind _output_get (Variables|Default|SetWeaponActor _returnvalue))
  (Transformation|AttachComponentToComponent _output_get (Variables|Character|GetMesh) "hand_r_rifle_socket" "SnapToTarget" "SnapToTarget" "SnapToTarget" true)
  (Variables|Default|SetWieldingWeapon true)
  (Default|CallOnWeaponEquipped))

(fn ConstructionScript
  (|CallParentFunction))

(fn GetIdealRange
  (return 6e+02 6e+02))

(fn SetMovementSpeed
  (params (Speed :type E_MovementSpeed%20Enum :default "NewEnumerator0"))
  (bind _output_get (Variables|/Script/Engine.CharacterMovementComponent|SetMaxWalkSpeed (Variables|Character|GetCharacterMovement) (Utilities|Select :Index Speed :NewEnumerator0 0.0 :NewEnumerator1 2e+02 :NewEnumerator2 3e+02 :NewEnumerator3 5e+02)))
  (return _output_get))