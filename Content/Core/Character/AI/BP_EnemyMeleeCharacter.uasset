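; Sword-wielding melee AI enemy with slash, leaping and spinning-chase attacks, weapon equip/unequip and chance-based blocking; the default Attack uses the slash.
; Montage notifies trigger sphere-trace damage through the attacks component, sword spawning, leaps and spins, with interruption disabled during attacks.
; Leaps launch along an arc toward the target's predicted position; spins rotate the mesh by timeline.
; Blockable hits may start a timed block before reaching the damage component.
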(event OnBlocked(BP_DamageSystemComponent)
  (params (CanBeParried :type Boolean))
  ;[1 1 1] Blocking
  (Variables|Default|SetBlockingState "NewEnumerator2")
  (Utilities|Time|ClearandInvalidateTimerbyHandle (Variables|Default|GetHoldBlockTimer))
  (Animation|Montage|PlayMontage (Variables|Character|GetMesh) "/Game/Mannequin/Animations/AM_BlockReaction_2Hands.AM_BlockReaction_2Hands"
    (:OnCompleted
      (CallFunction|EndBlock))
    (:OnInterrupted
      (CallFunction|EndBlock))))

(event Custom|StartBlock
  ;[1 1 1] Blocking
  (Utilities|Time|ClearandInvalidateTimerbyHandle (Variables|Default|GetHoldBlockTimer))
  (Components|Movement|StopMovementImmediately (Variables|Character|GetCharacterMovement))
  (Variables|/Game/Gameplay/DamageSystem/BP_DamageSystemComponent.BP_DamageSystemComponent_C|SetIsBlocking (Variables|Default|GetBP_DamageSystemComponent) true)
  (Variables|Default|SetBlockingState "NewEnumerator1")
  (bind _returnvalue (Utilities|Time|SetTimerbyEvent (EventDispatchers|CreateEvent :!event Custom|EndBlock) 2.0))
  (Variables|Default|SetHoldBlockTimer _returnvalue))

(event Custom|EndBlock
  ;[1 1 1] Blocking
  (Variables|/Game/Gameplay/DamageSystem/BP_DamageSystemComponent.BP_DamageSystemComponent_C|SetIsBlocking (Variables|Default|GetBP_DamageSystemComponent) false)
  (Variables|Default|SetBlockingState "NewEnumerator0")
  (Default|CallOnBlockEnded))

(event Custom|LongRangeAttack
  (params (AttackTarget :type Actor%20Object%20Reference))
  (|CallParentFunction AttackTarget)
  (bind _notifyname (Animation|Montage|PlayMontage (Variables|Character|GetMesh) "/Game/Mannequin/Animations/AM_JumpAttack_SwordShield_Montage.AM_JumpAttack_SwordShield_Montage")
    (:then
      (Variables|/Game/Gameplay/DamageSystem/BP_DamageSystemComponent.BP_DamageSystemComponent_C|SetIsInterruptible (Variables|Default|GetBP_DamageSystemComponent) false))
    (:OnCompleted
      (CallFunction|AttackEnd AttackTarget :!label _label)
      (Variables|/Game/Gameplay/DamageSystem/BP_DamageSystemComponent.BP_DamageSystemComponent_C|SetIsInterruptible (Variables|Default|GetBP_DamageSystemComponent) true))
    (:OnInterrupted
      (goto _label))
    (:OnNotifyBegin
      (switch name _notifyname
        (:Slash
          (Utilities|SphereTraceDamage))
        (:Jump
          (Utilities|JumptoAttackTarget AttackTarget))))))

(event Custom|ShortRangeAttack
  (params (AttackTarget :type Actor%20Object%20Reference))
  (|CallParentFunction AttackTarget)
  (bind _notifyname (Animation|Montage|PlayMontage (Variables|Character|GetMesh) "/Game/Mannequin/Animations/AM_SwordSlash_Montage.AM_SwordSlash_Montage")
    (:then
      (Variables|/Game/Gameplay/DamageSystem/BP_DamageSystemComponent.BP_DamageSystemComponent_C|SetIsInterruptible (Variables|Default|GetBP_DamageSystemComponent) false))
    (:OnCompleted
      (CallFunction|AttackEnd AttackTarget :!label _label)
      (Variables|/Game/Gameplay/DamageSystem/BP_DamageSystemComponent.BP_DamageSystemComponent_C|SetIsInterruptible (Variables|Default|GetBP_DamageSystemComponent) true))
    (:OnInterrupted
      (goto _label))
    (:OnNotifyBegin
      (switch name _notifyname
        (:Slash
          (Utilities|SphereTraceDamage))))))

(event Custom|SpinningAttack
  (params (AttackTarget :type Actor%20Object%20Reference))
  (|CallParentFunction AttackTarget)
  (bind _notifyname (Animation|Montage|PlayMontage (Variables|Character|GetMesh) "/Game/Mannequin/Animations/AM_SpinningAttack_Sword.AM_SpinningAttack_Sword")
    (:then
      (Variables|/Game/Gameplay/DamageSystem/BP_DamageSystemComponent.BP_DamageSystemComponent_C|SetIsInterruptible (Variables|Default|GetBP_DamageSystemComponent) false))
    (:OnCompleted
      (CallFunction|AttackEnd AttackTarget :!label _label)
      (Variables|/Game/Gameplay/DamageSystem/BP_DamageSystemComponent.BP_DamageSystemComponent_C|SetIsInterruptible (Variables|Default|GetBP_DamageSystemComponent) true)
      (CallFunction|StopSpinning))
    (:OnInterrupted
      (goto _label))
    (:OnNotifyBegin
      (switch name _notifyname
        (:Slash
          (Utilities|SphereTraceDamage))
        (:Spin
          (CallFunction|SpinMesh)
          (CallFunction|ChaseAttackTarget AttackTarget))))))

(event Custom|SpinMesh
  ;[1 1 1] Attack helpers
  (Variables|Default|SetMeshRotationBeforeSpin (Variables|/Script/Engine.SceneComponent|GetRelativeRotation (Variables|Character|GetMesh)))
  (bind _zrotationalpha (Timeline|SpinMeshTimeline PlayFromStart)
    (:Update
      (Transformation|SetRelativeRotation (Variables|Character|GetMesh) (Math|Rotator|MakeRotator (.roll (Variables|Default|GetMeshRotationBeforeSpin)) (.pitch (Variables|Default|GetMeshRotationBeforeSpin)) (Math|Float|Lerp (.yaw (Variables|Default|GetMeshRotationBeforeSpin)) (+ (.yaw (Variables|Default|GetMeshRotationBeforeSpin)) (|(360*12))) _zrotationalpha)) false false))))

(event Custom|StopSpinning
  ;[1 1 1] Attack helpers
  (Audio|Components|Audio|Stop (Variables|Default|GetSpinMeshTimeline))
  (Transformation|SetRelativeRotation (Variables|Character|GetMesh) (Variables|Default|GetMeshRotationBeforeSpin) false false))

(event Custom|ChaseAttackTarget
  (params (AttackTarget :type Actor%20Object%20Reference))
  ;[1 1 1] Attack helpers
  (AI|AIMoveTo self "0, 0, 0" AttackTarget 2e+02 false
    (:OnSuccess
      (Utilities|FlowControl|Delay 0.1)
      (if (Variables|Default|GetAttacking)
        (CallFunction|ChaseAttackTarget AttackTarget)))))

(event EventBeginPlay
  (|CallParentFunction)
  (Utilities|FlowControl|Sequence
    (:then_0
      (Variables|Default|SetMeshRotationBeforeSpin (Variables|/Script/Engine.SceneComponent|GetRelativeRotation (Variables|Character|GetMesh))))))

(event EventUnequipWeapon
  (bind _notifyname (Animation|Montage|PlayMontage (Variables|Character|GetMesh) "/Game/Mannequin/Animations/AM_SwordSheath_Montage.AM_SwordSheath_Montage")
    (:OnCompleted
      (Default|CallOnWeaponUnequipped)
      (Development|PrintString "Knife sheathed!"))
    (:OnNotifyBegin
      (switch name _notifyname
        (:UnholdSword
          (Actor|DestroyActor (Variables|Default|GetWeaponActor))
          (Variables|Default|SetWieldingWeapon false))))))

(event EventEquipWeapon
  (bind _notifyname (Animation|Montage|PlayMontage (Variables|Character|GetMesh) "/Game/Mannequin/Animations/AM_SwordWithdraw_Montage.AM_SwordWithdraw_Montage")
    (:OnCompleted
      (Development|PrintString "Sword wielded!"))
    (:OnNotifyBegin
      (switch name _notifyname
        (:HoldSword
          (bind _returnvalue (Game|SpawnActorfromClass "/Game/Gameplay/Weapons/BP_WeaponSword.BP_WeaponSword_C" (Transformation|GetActorTransform) "Undefined" "MultiplyWithRoot" 0 0))
          (bind _output_get (Variables|Default|SetWeaponActor _returnvalue))
          (Transformation|AttachComponentToComponent _output_get (Variables|Character|GetMesh) "hand_r_sword_socket" "SnapToTarget" "SnapToTarget" "SnapToTarget" true)
          (Variables|Default|SetWieldingWeapon true)
          (Default|CallOnWeaponEquipped))))))

(event EventAttack
  (params (AttackTarget :type Actor%20Object%20Reference))
  (CallFunction|ShortRangeAttack AttackTarget))

(fn ConstructionScript
  (|CallParentFunction))

(fn TakeDamage
  (params (DamageInfo :type S%20Damage%20Info%20Structure) (DamageCauser :type Actor%20Object%20Reference))
  (if (.CanBeBlocked (Utilities|Struct|BreakS_DamageInfo DamageInfo))
    (CallFunction|TrytoBlock)
    (bind _wasdamaged (Default|TakeDamage (Variables|Default|GetBP_DamageSystemComponent) DamageInfo DamageCauser))
    (return _wasdamaged)
    (else
      (bind _wasdamaged_2 (Default|TakeDamage (Variables|Default|GetBP_DamageSystemComponent) DamageInfo DamageCauser))
      (return _wasdamaged_2))))

(fn TrytoBlock
  (if (<= (Math|Random|RandomFloat) (Variables|Default|GetBlockChance))
    (CallFunction|StartBlock)))

(fn GetIdealRange
  (return 2e+02 4e+02))

(fn PredictActorLocation
  (params (Actor :type Actor%20Object%20Reference) (Time :type Float%20%28double-precision%29))
  (return (+ (Transformation|GetActorLocation Actor) (* Time (* (Transformation|GetVelocity Actor) "1.000000,1.000000,0.000000")))))

(event Custom|OnCharacterLanded
  (params (Hit :type Hit%20Result%20Structure%20%28by%20ref%29))
  (EventDispatchers|UnbindEventfromLandedDelegate (delegate Custom|OnCharacterLanded))
  (Components|Movement|StopMovementImmediately (Variables|Character|GetCharacterMovement)))