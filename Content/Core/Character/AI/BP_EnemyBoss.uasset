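; BP_EnemyBoss is a boss enemy character that wields an axe and has its own boss health bar.
; BeginPlay sets up health, clears the inherited health bar widget and creates a WBP_BossHealthBar, which the TakeDamage override refreshes.
; Equip and unequip spawn or destroy the hand-socketed axe, firing completion dispatchers a tick later.
; AttackCombo1 sends a blockable, parryable montage attack to the attacks component, and SetMovementSpeed maps speed states to walk speed.
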(event Custom|AttackCombo1
  (params (AttackTarget :type Actor%20Object%20Reference))
  (Default|PrimaryMeleeAttack (Variables|Default|GetBP_AttacksComponent) (Utilities|Struct|MakeS_AttackInfo AttackTarget "/Game/Mannequin/Animations/AM_ComboAttack_Axe.AM_ComboAttack_Axe" (Utilities|Struct|MakeS_DamageInfo 2e+01 "NewEnumerator1" "NewEnumerator1" false true true)) 4e+01 2.2e+02))

(event EventBeginPlay
  (bind _bp_damagesystemcomponent (Variables|Default|GetBP_DamageSystemComponent))
  (bind _bp_damagesystemcomponent_2 (Variables|Default|GetBP_DamageSystemComponent))
  (|CallParentFunction)
  (Utilities|FlowControl|Sequence
    (:then_0
      (bind _output_get (Variables|/Game/Gameplay/DamageSystem/BP_DamageSystemComponent.BP_DamageSystemComponent_C|SetMaxHealth _bp_damagesystemcomponent (Variables|Default|GetMax%20Health)))
      (Variables|/Game/Gameplay/DamageSystem/BP_DamageSystemComponent.BP_DamageSystemComponent_C|SetHealth _bp_damagesystemcomponent _output_get))
    (:then_1
      (UserInterface|SetWidget (Variables|Default|GetHealthBarWidget) 0)
      (bind _returnvalue (UserInterface|CreateWidget "/Game/UI/Widgets/WBP_BossHealthBar.WBP_BossHealthBar_C"))
      (bind _output_get_2 (Variables|Default|SetBossHealthBarWidget _returnvalue))
      (Default|UpdateHealthPercentage _output_get_2 (Variables|/Game/Gameplay/DamageSystem/BP_DamageSystemComponent.BP_DamageSystemComponent_C|GetHealth _bp_damagesystemcomponent_2) (Variables|/Game/Gameplay/DamageSystem/BP_DamageSystemComponent.BP_DamageSystemComponent_C|GetMaxHealth _bp_damagesystemcomponent_2)))))

(event EventEquipWeapon
  (bind _returnvalue (Game|SpawnActorfromClass "/Game/Gameplay/Weapons/BP_WeaponAxe.BP_WeaponAxe_C" (Math|Transform|MakeTransform "0, 0, 0" "0, 0, 0" "1.000000,1.000000,1.000000") "Undefined" "MultiplyWithRoot" 0 0))
  (bind _output_get (Variables|Default|SetWeaponActor _returnvalue))
  (Transformation|AttachComponentToComponent _output_get (Variables|Character|GetMesh) "hand_r_axe_socket" "SnapToTarget" "SnapToTarget" "SnapToTarget" true)
  (Variables|Default|SetWieldingWeapon true)
  (Utilities|FlowControl|DelayUntilNextTick)
  (Default|CallOnWeaponEquipped))

(event EventUnequipWeapon
  (Actor|DestroyActor (Variables|Default|GetWeaponActor))
  (Variables|Default|SetWieldingWeapon false)
  (Utilities|FlowControl|DelayUntilNextTick)
  (Default|CallOnWeaponUnequipped))

(fn ConstructionScript
  (|CallParentFunction))

(fn SetMovementSpeed
  (params (Speed :type E_MovementSpeed%20Enum :default "NewEnumerator0"))
  (bind _output_get (Variables|/Script/Engine.CharacterMovementComponent|SetMaxWalkSpeed (Variables|Character|GetCharacterMovement) (Utilities|Select :Index Speed :NewEnumerator0 0.0 :NewEnumerator1 1e+02 :NewEnumerator2 2e+02 :NewEnumerator3 3.5e+02)))
  (return _output_get))

(fn TakeDamage
  (params (DamageInfo :type S%20Damage%20Info%20Structure) (DamageCauser :type Actor%20Object%20Reference))
  (bind _bp_damagesystemcomponent (Variables|Default|GetBP_DamageSystemComponent))
  (bind _wasdamaged (|CallParentFunction DamageInfo DamageCauser))
  (Default|UpdateHealthPercentage (Variables|Default|GetBossHealthBarWidget) (Variables|/Game/Gameplay/DamageSystem/BP_DamageSystemComponent.BP_DamageSystemComponent_C|GetHealth _bp_damagesystemcomponent) (Variables|/Game/Gameplay/DamageSystem/BP_DamageSystemComponent.BP_DamageSystemComponent_C|GetMaxHealth _bp_damagesystemcomponent))
  (return _wasdamaged))