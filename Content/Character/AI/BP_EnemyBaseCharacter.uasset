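; Base enemy character that links an AI controller, a shared damage component and a health bar widget.
; On BeginPlay it caches its enemy AI controller, creates the health bar for itself and binds the death event.
; Death enables ragdoll physics, stops the behavior logic and sets the controller state to dead.
; Functions forward health and damage calls to the component and supply patrol route, combat ranges and speed presets.
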(event Custom|OnDeath
  (bind _mesh (Variables|Character|GetMesh))
  (Physics|SetSimulatePhysics _mesh true)
  (Collision|SetCollisionEnabled _mesh "QueryAndPhysics")
  (AI|Logic|StopLogic (Variables|/Script/AIModule.AIController|GetBrainComponent (Variables|Default|GetAIC_EnemyBase)) "")
  (Default|SetStateasDead (Variables|Default|GetAIC_EnemyBase)))

(event EventBeginPlay
  (Utilities|FlowControl|Sequence
    (:then_0
      (bind _asaic_enemy_base (Utilities|Casting|CastToAIC_EnemyBase (AI|GetAIController self)))
      (Variables|Default|SetAIC_EnemyBase _asaic_enemy_base))
    (:then_1
      (bind _returnvalue (UserInterface|CreateWidget "/Game/UI/WBP_HealthBar.WBP_HealthBar_C" 0 self))
      (UserInterface|SetWidget (Variables|Default|GetHealthBarWidget) _returnvalue))
    (:then_2
      (EventDispatchers|AssignOnDeath (Variables|Default|GetBP_DamageSystemComponent) (EventDispatchers|CreateEvent :!event Custom|OnDeath)))))

(fn ConstructionScript)

(fn GetCurrentHealth
  (return (Variables|/Game/Gameplay/DamageSystem/BP_DamageSystemComponent.BP_DamageSystemComponent_C|GetHealth (Variables|Default|GetBP_DamageSystemComponent))))

(fn GetIdealRange
  (return 1.5e+02 3.5e+02))

(fn GetMaxHealth
  (return (Variables|/Game/Gameplay/DamageSystem/BP_DamageSystemComponent.BP_DamageSystemComponent_C|GetMaxHealth (Variables|Default|GetBP_DamageSystemComponent))))

(fn GetPatrolRoute
  (return (Variables|AI|GetPatrolRoute)))

(fn Heal
  (params (Amount :type Float%20%28double-precision%29))
  (bind _newhealth (Default|Heal (Variables|Default|GetBP_DamageSystemComponent) Amount))
  (return _newhealth))

(fn IsDead
  (return (Variables|/Game/Gameplay/DamageSystem/BP_DamageSystemComponent.BP_DamageSystemComponent_C|GetIsDead (Variables|Default|GetBP_DamageSystemComponent))))

(fn SetMovementSpeed
  (params (Speed :type E_MovementSpeed%20Enum :default "NewEnumerator0"))
  (bind _output_get (Variables|/Script/Engine.CharacterMovementComponent|SetMaxWalkSpeed (Variables|Character|GetCharacterMovement) (Utilities|Select :Index Speed :NewEnumerator0 0.0 :NewEnumerator1 1e+02 :NewEnumerator2 3e+02 :NewEnumerator3 5e+02)))
  (return _output_get))

(fn TakeDamage
  (params (DamageInfo :type S%20Damage%20Info%20Structure))
  (bind _wasdamaged (Default|TakeDamage (Variables|Default|GetBP_DamageSystemComponent) DamageInfo))
  (return _wasdamaged))