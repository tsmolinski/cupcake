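; Ranged enemy character that spawns a rifle on BeginPlay and attaches it to its hand socket.
; Attack plays a rifle fire montage, and its notify traces on Visibility from the weapon to the AI controller's attack target.
; Damage is sent to the target via a message only when that trace hits nothing.
; It also supplies its ideal attack and defend range and maps movement states to walk speeds.
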(event EventBeginPlay
  (|CallParentFunction)
  (CallFunction|EquipWeapon))

(event EventAttack
  (bind _notifyname (Animation|Montage|PlayMontage (Variables|Character|GetMesh) "/Game/Mannequin/Animations/AM_Fire_Rifle_Ironsights.AM_Fire_Rifle_Ironsights")
    (:OnCompleted
      (Default|CallOnAttackEnd :!label _label))
    (:OnInterrupted
      (goto _label))
    (:OnNotifyBegin
      (switch name _notifyname
        (:Fire
          (bind _asaic_enemy_base (Utilities|Casting|CastToAIC_EnemyBase (AI|GetAIController self)))
          (Utilities|IsValid (Variables|/Game/Gameplay/AI/Controller/AIC_EnemyBase.AIC_EnemyBase_C|GetAttackTarget _asaic_enemy_base)
            (:Is%20Valid
              (bind _returnvalue (Collision|LineTraceByChannel (Transformation|GetActorLocation (Variables|Default|GetWeaponActor)) (Transformation|GetActorLocation (Variables|/Game/Gameplay/AI/Controller/AIC_EnemyBase.AIC_EnemyBase_C|GetAttackTarget _asaic_enemy_base)) "TraceTypeQuery1" false 0 "ForDuration"))
              (if (not _returnvalue)
                (Class|BPIDamagable|TakeDamage(Message) (Variables|/Game/Gameplay/AI/Controller/AIC_EnemyBase.AIC_EnemyBase_C|GetAttackTarget _asaic_enemy_base) (Utilities|Struct|MakeS_DamageInfo 2e+01 "NewEnumerator2"))))))))))

(event EventEquipWeapon
  (bind _returnvalue (Game|SpawnActorfromClass "/Game/Gameplay/Weapons/BP_WeaponRifle.BP_WeaponRifle_C" (Math|Transform|MakeTransform "0, 0, 0") "Undefined" "MultiplyWithRoot" 0 0))
  (bind _output_get (Variables|Default|SetWeaponActor _returnvalue))
  (Transformation|AttachComponentToComponent _output_get (Variables|Character|GetMesh) "hand_r_rifle_socket" "SnapToTarget" "SnapToTarget" "SnapToTarget" true)
  (Variables|Default|SetWieldingWeapon true)
  (Default|CallOnWeaponEquipped))

(fn ConstructionScript
  (|CallParentFunction))

(fn GetIdealRange
  (return 6e+02 6e+02))

(fn SetMovementSpeed
  (params (Speed :type E_MovementSpeed%20Enum :default "NewEnumerator0"))
  (bind _output_get (Variables|/Script/Engine.CharacterMovementComponent|SetMaxWalkSpeed (Variables|Character|GetCharacterMovement) (Utilities|Select :Index Speed :NewEnumerator0 0.0 :NewEnumerator1 2e+02 :NewEnumerator2 3e+02 :NewEnumerator3 5e+02)))
  (return _output_get))