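; Melee enemy AI character whose attack, weapon equip and block actions are montage-driven and signal their ends via event calls.
; Montage notifies time the sphere-trace damage and weapon spawn/destroy, using rifle assets as the knife; the trace end omits the actor location offset.
; Attacks are uninterruptible through the damage system component, whose OnBlocked event plays a block reaction, with a blocking state keeping the interrupted block montage from ending the block early.
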(event OnBlocked(BP_DamageSystemComponent)
  (params (CanBeParried :type Boolean))
  ;[1 1 1] Blocking
  (Variables|Default|SetBlockingState "NewEnumerator2")
  (Animation|Montage|PlayMontage (Variables|Character|GetMesh) "/Game/Mannequin/Animations/AM_BlockReaction_2Hands.AM_BlockReaction_2Hands"
    (:OnCompleted
      (CallFunction|EndBlock))
    (:OnInterrupted
      (CallFunction|EndBlock))))

(event Custom|StartBlock
  ;[1 1 1] Blocking
  (Components|Movement|StopMovementImmediately (Variables|Character|GetCharacterMovement))
  (Variables|/Game/Gameplay/DamageSystem/BP_DamageSystemComponent.BP_DamageSystemComponent_C|SetIsBlocking (Variables|Default|GetBP_DamageSystemComponent) true)
  (Variables|Default|SetBlockingState "NewEnumerator1")
  (Animation|Montage|PlayMontage (Variables|Character|GetMesh) "/Game/Mannequin/Animations/AM_Block_2Hands.AM_Block_2Hands"
    (:OnCompleted
      (CallFunction|EndBlock))
    (:OnInterrupted
      (if (Utilities|Enum|NotEqual(Enum) (Variables|Default|GetBlockingState) "NewEnumerator2")
        (CallFunction|EndBlock)))))

(event Custom|EndBlock
  ;[1 1 1] Blocking
  (Variables|/Game/Gameplay/DamageSystem/BP_DamageSystemComponent.BP_DamageSystemComponent_C|SetIsBlocking (Variables|Default|GetBP_DamageSystemComponent) false)
  (Variables|Default|SetBlockingState "NewEnumerator0")
  (Default|CallOnBlockEnded))

(event EventBeginPlay
  (|CallParentFunction) ; This node is disabled and will not be called.\nDrag off pins to build functionality.
)

(event EventUnequipWeapon
  (bind _notifyname (Animation|Montage|PlayMontage (Variables|Character|GetMesh) "/Game/AnimStarterPack/Equip_Rifle_Standing_Montage.Equip_Rifle_Standing_Montage")
    (:OnCompleted
      (Default|CallOnWeaponUnequipped)
      (Development|PrintString "Knife sheathed!"))
    (:OnNotifyBegin
      (switch name _notifyname
        (:HoldRife
          (Actor|DestroyActor (Variables|Default|GetWeaponActor))
          (Variables|Default|SetWieldingWeapon false))))))

(event EventEquipWeapon
  (bind _notifyname (Animation|Montage|PlayMontage (Variables|Character|GetMesh) "/Game/AnimStarterPack/Equip_Rifle_Standing_Montage.Equip_Rifle_Standing_Montage")
    (:OnCompleted
      (Development|PrintString "Knife wielded!"))
    (:OnNotifyBegin
      (switch name _notifyname
        (:HoldRife
          (bind _returnvalue (Game|SpawnActorfromClass "/Game/Gameplay/Weapons/BP_WeaponRifle.BP_WeaponRifle_C" (Transformation|GetActorTransform) "Undefined" "MultiplyWithRoot" 0 0))
          (bind _output_get (Variables|Default|SetWeaponActor _returnvalue))
          (Transformation|AttachComponentToComponent _output_get (Variables|Character|GetMesh) "hand_r_rifle_socket" "SnapToTarget" "SnapToTarget" "SnapToTarget" true)
          (Variables|Default|SetWieldingWeapon true)
          (Default|CallOnWeaponEquipped))))))

(event EventAttack
  (bind _notifyname (Animation|Montage|PlayMontage (Variables|Character|GetMesh) "/Game/Mannequin/Animations/AM_Fire_Rifle_Ironsights.AM_Fire_Rifle_Ironsights")
    (:then
      (Variables|/Game/Gameplay/DamageSystem/BP_DamageSystemComponent.BP_DamageSystemComponent_C|SetIsInterruptible (Variables|Default|GetBP_DamageSystemComponent) false))
    (:OnCompleted
      (Default|CallOnAttackEnd :!label _label)
      (Variables|/Game/Gameplay/DamageSystem/BP_DamageSystemComponent.BP_DamageSystemComponent_C|SetIsInterruptible (Variables|Default|GetBP_DamageSystemComponent) true)
      (Development|PrintString "Melee Attack!"))
    (:OnInterrupted
      (goto _label))
    (:OnNotifyBegin
      (switch name _notifyname
        (:Fire
          (bind (_outhit _returnvalue) (Collision|SphereTraceForObjects (Transformation|GetActorLocation) (* (Transformation|GetActorForwardVector) (Variables|Default|GetRange)) 2e+01 (Utilities|Array|MakeArray "ObjectTypeQuery3") false 0 "ForDuration"))
          (if _returnvalue
            (Class|BPIDamagable|TakeDamage(Message) (.HitActor (Collision|BreakHitResult _outhit)) (Utilities|Struct|MakeS_DamageInfo 25.0 "NewEnumerator1") self)))))))

(fn ConstructionScript
  (|CallParentFunction))