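; BP_AttacksComponent is an attack component that gives its owner a test projectile attack and a hitscan bullet attack.
; ShootProjectileTest spawns a targeted projectile ignoring the owner; its impact applies damage and calls OnAttackEnded.
; FireBullet line-traces Pawn objects with debug drawing and applies damage without checking for a hit.
; Both send damage through TakeDamageMessage and report damage events at the owner's location for AI sensing.
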(event Custom|ShootProjectileTest
  (params (SpawnTransform :type Transform) (Target :type Actor%20Object%20Reference) (DamageInfo :type S%20Damage%20Info%20Structure))
  (bind _returnvalue (Game|SpawnActorfromClass "/Game/Gameplay/Projectiles/BP_ProjectileTest.BP_ProjectileTest_C" SpawnTransform "Undefined" "MultiplyWithRoot" (Components|GetOwner) 1e+03 0.0 Target false 2e+03 0))
  (EventDispatchers|BindEventtoOnProjectileImpact _returnvalue (delegate Custom|OnProjectileImpacted))
  (Collision|IgnoreActorwhenMoving (Variables|/Game/Gameplay/Projectiles/BP_ProjectileBase.BP_ProjectileBase_C|GetBox _returnvalue) (Components|GetOwner) true))

(event Custom|OnProjectileImpacted
  (params (OtherActror :type Actor%20Object%20Reference) (Hit :type Hit%20Result%20Structure))
  (bind _returnvalue (Components|GetOwner))
  (Class|BPIDamagable|TakeDamage(Message) OtherActror (stale Custom|ShootProjectileTest DamageInfo))
  (Class|AISenseDamage|ReportDamageEvent OtherActror _returnvalue (.Amount (Utilities|Struct|BreakS_DamageInfo (stale Custom|ShootProjectileTest DamageInfo))) (Transformation|GetActorLocation _returnvalue) "0, 0, 0" "None")
  (Default|CallOnAttackEnded))

(event Custom|FireBullet
  (params (TraceStart :type Vector) (TraceEnd :type Vector) (DamageInfo :type S%20Damage%20Info%20Structure))
  (bind _returnvalue (Components|GetOwner))
  (bind _outhit (Collision|LineTraceForObjects TraceStart TraceEnd (Utilities|Array|MakeArray "ObjectTypeQuery3") false 0 "ForDuration"))
  (if (not false)
    (Class|BPIDamagable|TakeDamage(Message) (.HitActor (Collision|BreakHitResult _outhit)) DamageInfo)
    (Class|AISenseDamage|ReportDamageEvent (.HitActor (Collision|BreakHitResult _outhit)) _returnvalue (.Amount (Utilities|Struct|BreakS_DamageInfo DamageInfo)) (Transformation|GetActorLocation _returnvalue) "0, 0, 0" "None")))

(event EventBeginPlay)

(event EventTick
  (params (DeltaSeconds :type Float%20%28single-precision%29)))