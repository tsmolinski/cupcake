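; Base projectile actor that flies via a ProjectileMovement component, optionally homing on a Target, and reports what it hits.
; On BeginPlay it applies speed and gravity, makes its Box ignore the instigator (or owner), and aims velocity at any valid Target, adding homing if enabled.
; A Box hit calls OnProjectileImpact with the actor and hit data, plays impact effect and sound, then destroys the projectile.
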(event OnComponentHit(Box)
  (params (HitComponent :type Primitive%20Component%20Object%20Reference) (OtherActor :type Actor%20Object%20Reference) (OtherComp :type Primitive%20Component%20Object%20Reference) (NormalImpulse :type Vector :default "0, 0, 0") (Hit :type Hit%20Result%20Structure%20%28by%20ref%29))
  (bind _location (Collision|BreakHitResult Hit))
  (Default|CallOnProjectileImpact OtherActor Hit)
  (Effects|SpawnEmitteratLocation (Variables|Effects|GetImpactEffect) _location)
  (Audio|PlaySoundatLocation (Variables|Sounds|GetImpactSound) _location "0, 0, 0" 1.0 1.0 0.0 0 0 0 0)
  (Actor|DestroyActor))

(event Custom|RotateToTarget
  (Variables|/Script/Engine.MovementComponent|SetVelocity (Variables|Default|GetProjectileMovement) (* (Math|Vector|GetUnitDirection(Vector) (Transformation|GetActorLocation) (Transformation|GetActorLocation (Variables|Target|GetTarget))) (Variables|ProjectileSettings|GetSpeed))))

(event EventBeginPlay
  (bind _returnvalue (Game|GetInstigator))
  (bind _projectilemovement (Variables|Default|GetProjectileMovement))
  (bind _projectilemovement_2 (Variables|Default|GetProjectileMovement))
  (Utilities|FlowControl|Sequence
    (:then_0
      (Variables|/Script/Engine.ProjectileMovementComponent|SetInitialSpeed _projectilemovement (Variables|ProjectileSettings|GetSpeed))
      (Variables|/Script/Engine.ProjectileMovementComponent|SetMaxSpeed _projectilemovement (Variables|ProjectileSettings|GetSpeed))
      (Variables|/Script/Engine.ProjectileMovementComponent|SetProjectileGravityScale _projectilemovement (Variables|ProjectileSettings|GetGravity))
      (Variables|Target|GetTarget
        (:then
          (if (Variables|ProjectileSettings|GetIsHoming)
            (Variables|/Script/Engine.ProjectileMovementComponent|SetHomingAccelerationMagnitude _projectilemovement_2 (Variables|ProjectileSettings|GetHoming%20Acceleration%20Magnitude))
            (Variables|/Script/Engine.ProjectileMovementComponent|SetbIsHomingProjectile _projectilemovement_2 true)
            (Variables|/Script/Engine.ProjectileMovementComponent|SetHomingTargetComponent _projectilemovement_2 (Variables|/Script/Engine.Actor|GetRootComponent (Variables|Target|GetTarget)))))
        (:else)))
    (:then_1
      (Collision|IgnoreActorwhenMoving (Variables|Default|GetBox) (select (Utilities|IsValid _returnvalue) _returnvalue (Components|GetOwner)) true))
    (:then_2
      (Variables|Target|GetTarget
        (:then
          (CallFunction|RotatetoTarget))
        (:else)))))

(fn ConstructionScript)